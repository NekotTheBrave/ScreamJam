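; HealthPickup is an interactable pickup actor that adds a health kit to the first-person character's inventory count.
; Its Interact event checks that the interactor implements InteractInterface, casts it to BP_FirstPersonCharacter, increments HealthKits and destroys the pickup.
; A sphere swaps the mesh material when an interface-implementing actor begins overlapping, and restores MI_Ground when any overlap ends.
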(event `/Game/CustomContent/Blueprints/InteractInterface.Interact`
  (params (Interactor :type "Actor Object Reference"))
  (`KismetSystemLibrary.PrintString` "Hello")
  (if (`KismetSystemLibrary.DoesImplementInterface` Interactor "/Game/CustomContent/Blueprints/InteractInterface.InteractInterface_C")
    (bind _asbp_first_person_character (cast `/Game/CustomContent/Blueprints/BP_FirstPersonCharacter` Interactor)
      (:`then`
        (bind _result (`/Engine/EditorBlueprintResources/StandardMacros.IncrementInt` (`/Game/CustomContent/Blueprints/BP_FirstPersonCharacter.HealthKits` _asbp_first_person_character))
          (:`  `
            (set `/Game/CustomContent/Blueprints/BP_FirstPersonCharacter.HealthKits` _result _asbp_first_person_character)
            (`self.K2_DestroyActor`))))
      (:`CastFailed`
        (`KismetSystemLibrary.PrintString` "failed to pick up")))))

(event `self.Sphere.OnComponentBeginOverlap`
  (params (OverlappedComponent :type "PrimitiveComponent Object Reference") (OtherActor :type "Actor Object Reference") (OtherComp :type "PrimitiveComponent Object Reference") (OtherBodyIndex :type Integer) (bFromSweep :type Boolean) (SweepResult :type "HitResult Structure (by ref)"))
  (if (`KismetSystemLibrary.DoesImplementInterface` OtherActor "/Game/CustomContent/Blueprints/InteractInterface.InteractInterface_C")
    (`PrimitiveComponent.SetMaterial` (`self.StaticMesh`) 0 "/Game/CustomContent/Materials/MFI_Ground.MFI_Ground")))

(event `self.Sphere.OnComponentEndOverlap`
  (params (OverlappedComponent :type "PrimitiveComponent Object Reference") (OtherActor :type "Actor Object Reference") (OtherComp :type "PrimitiveComponent Object Reference") (OtherBodyIndex :type Integer))
  (`PrimitiveComponent.SetMaterial` (`self.StaticMesh`) 0 "/Game/CustomContent/Materials/MI_Ground.MI_Ground"))

(fn `UserConstructionScript`)