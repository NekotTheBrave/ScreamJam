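; Test door actor that slides vertically when interacted with, unless locked.
; Interact prints a debug message, then OpenDoor timeline moves the mesh, waits five seconds, and Timeline_0 moves it back.
; Movement accumulates world offsets per update; re-trigger guards cover opening and waiting, but not closing.
; Sphere overlap by InteractInterface actors swaps the mesh material; any end overlap restores it.
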(event `self.Sphere.OnComponentBeginOverlap`
  (params (OverlappedComponent :type "PrimitiveComponent Object Reference") (OtherActor :type "Actor Object Reference") (OtherComp :type "PrimitiveComponent Object Reference") (OtherBodyIndex :type Integer) (bFromSweep :type Boolean) (SweepResult :type "HitResult Structure (by ref)"))
  (if (`KismetSystemLibrary.DoesImplementInterface` OtherActor "/Game/CustomContent/Blueprints/InteractInterface.InteractInterface_C")
    (`PrimitiveComponent.SetMaterial` (`self.StaticMesh`) 0 "/Game/CustomContent/Materials/MFI_Ground.MFI_Ground")))

(event `self.Sphere.OnComponentEndOverlap`
  (params (OverlappedComponent :type "PrimitiveComponent Object Reference") (OtherActor :type "Actor Object Reference") (OtherComp :type "PrimitiveComponent Object Reference") (OtherBodyIndex :type Integer))
  (`PrimitiveComponent.SetMaterial` (`self.StaticMesh`) 0 "/Game/CustomContent/Materials/MI_Ground.MI_Ground"))

(event `self.Interact`
  (params (Interactor :type "Actor Object Reference"))
  (bind _staticmesh (`self.StaticMesh`))
  (`KismetSystemLibrary.PrintString` "Hello")
  (if (`KismetSystemLibrary.DoesImplementInterface` Interactor "/Game/CustomContent/Blueprints/InteractInterface.InteractInterface_C")
    (if (not (`self.IsLocked`))
      (if (and (not (`TimelineComponent.IsPlaying` (`self.OpenDoor`))) (not (`self.waiting`)))
        (bind (_direction _myfloattrack) (`Timeline|OpenDoor` :!via `PlayFromStart`)
          (:`Update`
            (`SceneComponent.K2_AddWorldOffset` _staticmesh (`KismetMathLibrary.MakeVector` 0.0 0.0 (* _myfloattrack 13.0)) false false))
          (:`Finished`
            (set `self.waiting` true)
            (`KismetSystemLibrary.Delay` 5.0)
            (set `self.waiting` false)
            (bind (_direction_2 _myfloattrack_2) (`Timeline|Timeline_0` :!via `ReverseFromEnd`)
              (:`Update`
                (`SceneComponent.K2_AddWorldOffset` _staticmesh (`KismetMathLibrary.MakeVector` 0.0 0.0 (* _myfloattrack_2 -13.0)) false false)))))))))

(fn `UserConstructionScript`)